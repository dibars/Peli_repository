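; Falling coin collectible that the player gathers by character overlap, touch or mouse click.
; BeginPlay and construction set vertical drop, scale and speed settings; movement is left to the parent Tick.
; Character overlap broadcasts the coin's Value, while touch and click add a fixed amount to PELI2_Variables' CollectedMoney and play a sound.
; Collection or hitting the respawn trigger recycles the coin by resetting position, scale, value and speed.
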(event OnClicked(PaperFlipbook)
  (params (TouchedComponent :type Primitive%20Component%20Object%20Reference) (ButtonPressed :type Key%20Structure :default "None"))
  ;[1 1 1] collect mcoins with mouse
  (bind _aspeli2_variables (Utilities|Casting|CastToPELI2_Variables (Game|GetGameInstance)))
  (Variables|/Game/Blueprints/PELI2_Variables.PELI2_Variables_C|SetCollectedMoney _aspeli2_variables (+ (Variables|/Game/Blueprints/PELI2_Variables.PELI2_Variables_C|GetCollectedMoney _aspeli2_variables) 5))
  (Audio|PlaySound2D "/Game/Audio/Pin_Drop-SoundBible_com-655931796.Pin_Drop-SoundBible_com-655931796" 1.0 1.0 0.0 0 0)
  (CallFunction|ResetPosition)
  (bind _returnvalue (Rendering|Material|GetVectorParameterValue 0 "None" :!class /Script/Engine.KismetMaterialLibrary))
  (CallFunction|SetSpeed)
  (CallFunction|ResetScaleandValue)
  (bind _returnvalue_2 (Rendering|Material|GetScalarParameterValue 0 "None" :!class /Script/Engine.KismetMaterialLibrary)))

(event OnInputTouchBegin(PaperFlipbook)
  (params (FingerIndex :type ETouchIndex%20Enum :default "Touch1") (TouchedComponent :type Primitive%20Component%20Object%20Reference))
  ;[1 1 1] Prints Hello, adds 5 coins to the meter and destroys itself when coin is clicked
  (bind _aspeli2_variables (Utilities|Casting|CastToPELI2_Variables (Game|GetGameInstance)))
  (Variables|/Game/Blueprints/PELI2_Variables.PELI2_Variables_C|SetCollectedMoney _aspeli2_variables (+ (Variables|/Game/Blueprints/PELI2_Variables.PELI2_Variables_C|GetCollectedMoney _aspeli2_variables) 5))
  (Audio|PlaySound2D "/Game/Audio/Pin_Drop-SoundBible_com-655931796.Pin_Drop-SoundBible_com-655931796" 1.0 1.0 0.0 0 0)
  (CallFunction|ResetPosition)
  (bind _returnvalue (Rendering|Material|GetVectorParameterValue 0 "None" :!class /Script/Engine.KismetMaterialLibrary))
  (CallFunction|SetSpeed)
  (CallFunction|ResetScaleandValue)
  (bind _returnvalue_2 (Rendering|Material|GetScalarParameterValue 0 "None" :!class /Script/Engine.KismetMaterialLibrary)))

(event Collision|EventActorBeginOverlap
  (params (OtherActor :type Actor%20Object%20Reference))
  (bind _returnvalue (Utilities|GetObjectName OtherActor))
  ;[1 1 1] Check if coin hit character
  (bind _hitresult (CallFunction|CheckCharHit _returnvalue))
  (if _hitresult
    ;[1 1 1] Broadcast message that money was collected
    (Default|CallMoneyCollectedED (Variables|Default|GetValue))
    ;[1 1 1] Resetting position, scale and value
    (CallFunction|ResetPosition :!label _label)
    (CallFunction|ResetScaleandValue)
    (CallFunction|SetSpeed)
    (else
      ;[1 1 1] If not char, check if we hit respawn trigger
      (bind _hitresult_2 (CallFunction|CheckRespawnHit _returnvalue))
      (if _hitresult_2
        (goto _label)))))

(event EventTick
  (params (DeltaSeconds :type Float%20%28single-precision%29))
  (|CallParentFunction 0.0))

(event EventBeginPlay
  ;[1 1 1] Liikkuuko vertikaalisesti
  (Variables|Default|SetDropsVertically true)
  ;[1 1 1] Määrittelee skaalauksen ja nopeuden vaihteluvälin ja liikkeen suunnan
  (Variables|Default|SetDefaultScale 3.0)
  (Variables|Default|SetMinScale 2.0)
  (Variables|Default|SetMaxScale 5.0)
  (Variables|Default|SetDefaultSpeed "0.000000, 0,-7.000000")
  (Variables|Default|SetSpeedVariance 2.0))

(fn ConstructionScript
  ;[1 1 1] Initial position ja speed
  (Variables|Default|SetSpeed "0, 0,-5.000000")
  (Variables|Default|SetInitialPosition "0,0.000000,1000.000000"))