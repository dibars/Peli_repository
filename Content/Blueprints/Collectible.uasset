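; Base collectible actor that drifts by a Speed vector each frame, scaled by truncated global time dilation rather than delta time.
; Helper functions randomize respawn position along X or Z (per DropsVertically), per-axis scale and speed, and set Value from the unrandomized default scale.
; Name-based checks identify player and respawn-trigger hits.
; ApplyEffect is an empty hook, and nothing in this Blueprint calls these functions.
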(event EventBeginPlay)

(event Collision|EventActorBeginOverlap
  (params (OtherActor :type Actor%20Object%20Reference)))

(event EventTick
  (params (DeltaSeconds :type Float%20%28single-precision%29))
  ;[1 1 1] Move the collectible
  (Transformation|AddActorWorldOffset (* (Variables|Default|GetSpeed) (Math|Float|Truncate (Class|GameplayStatics|GetGlobalTimeDilation)))))

(fn ConstructionScript)

(fn ResetPosition
  (bind _initialposition (Variables|Default|GetInitialPosition))
  (bind (_x _y _z) (Math|Vector|BreakVector _initialposition))
  (bind (_x_2 _y_2) (Math|Vector|BreakVector _initialposition))
  ;[1 1 1] Liikkuuko collectable vertikaalisesti vai horisontaalisesti
  (if (Variables|Default|GetDropsVertically)
    (Transformation|SetActorLocation (Math|Vector|MakeVector (Math|Random|RandomFloatinRange -5e+02 5e+02) _y _z) false false)
    (else
      (Transformation|SetActorLocation (Math|Vector|MakeVector _x_2 _y_2 (Math|Random|RandomFloatinRange 1.5e+02 8e+02)) false false))))

(fn ResetScaleandValue
  ;[1 1 1] Peruskoko collectable
  (bind _output_get (Variables|Default|SetScale (Variables|Default|GetDefaultScale)))
  (Transformation|SetActorScale3D (Math|Vector|MakeVector (/ _output_get (Math|Random|RandomFloatinRange (Variables|Default|GetMinScale) (Variables|Default|GetMaxScale))) (/ _output_get (Math|Random|RandomFloatinRange (Variables|Default|GetMinScale) (Variables|Default|GetMaxScale))) (/ _output_get (Math|Random|RandomFloatinRange (Variables|Default|GetMinScale) (Variables|Default|GetMaxScale)))))
  (Variables|Default|SetValue (Math|Float|Round (Variables|Default|GetScale))))

(fn CheckCharHit
  (params (OtherObjectName :type String))
  (return (Utilities|Enum|Equal(Enum) OtherObjectName (Utilities|GetObjectName (Game|GetPlayerCharacter 0)))))

(fn CheckRespawnHit
  (params (OtherObjectName :type String))
  (return (or (Utilities|Enum|Equal(Enum) OtherObjectName (Variables|Default|GetRespawnTriggerName)) (Utilities|Enum|Equal(Enum) OtherObjectName (Variables|Default|GetRespawnTriggerNameBottom)))))

(fn ApplyEffect)

(fn SetSpeed
  (bind _speedvariance (Variables|Default|GetSpeedVariance))
  (bind _defaultspeed (Variables|Default|GetDefaultSpeed))
  ;[1 1 1] Asettaa uuden nopeuden kertomalla DefaultSpeed SpeedVariance
  (Variables|Default|SetSpeed (* _defaultspeed (Math|Random|RandomFloatinRange (/ (Math|Vector|GetMaxElement _defaultspeed) _speedvariance) _speedvariance))))