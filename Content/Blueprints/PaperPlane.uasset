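; Paper plane actor that flies horizontally across the level and opens a QuestionUI widget with a button sound when its flipbook is tapped or clicked.
; BeginPlay and the construction script configure start position, speed, scale range and variance, while Tick defers to the parent class.
; Overlapping the character or respawn trigger resets its position, scale and value, then sets a new speed, recycling the same actor.
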(event OnClicked(PaperFlipbook1)
  (params (TouchedComponent :type Primitive%20Component%20Object%20Reference) (ButtonPressed :type Key%20Structure))
  (bind _returnvalue (UserInterface|CreateWidget "/Game/Blueprints/GUI/QuestionUI.QuestionUI_C"))
  (bind _output_get (Variables|Default|SetQuestionUiRef _returnvalue))
  (UserInterface|Viewport|AddtoViewport _output_get 0)
  (Audio|PlaySound2D "/Game/Audio/Tiny_Button_Push-SoundBible_com-513260752.Tiny_Button_Push-SoundBible_com-513260752" 1.0 1.0 0.0 0 0))

(event OnInputTouchBegin(PaperFlipbook1)
  (params (FingerIndex :type ETouchIndex%20Enum :default "Touch1") (TouchedComponent :type Primitive%20Component%20Object%20Reference))
  (bind _returnvalue (UserInterface|CreateWidget "/Game/Blueprints/GUI/QuestionUI.QuestionUI_C"))
  (bind _output_get (Variables|Default|SetQuestionUiRef _returnvalue))
  (UserInterface|Viewport|AddtoViewport _output_get 0)
  (Audio|PlaySound2D "/Game/Audio/Tiny_Button_Push-SoundBible_com-513260752.Tiny_Button_Push-SoundBible_com-513260752" 1.0 1.0 0.0 0 0))

(event Collision|EventActorBeginOverlap
  (params (OtherActor :type Actor%20Object%20Reference))
  (bind _returnvalue (Utilities|GetObjectName OtherActor))
  ;[1 1 1] Check if coin hit character
  (bind _hitresult (CallFunction|CheckCharHit _returnvalue))
  (if _hitresult
    ;[1 1 1] Resetting position, scale and value
    (CallFunction|ResetPosition :!label _label)
    (CallFunction|ResetScaleandValue)
    (CallFunction|SetSpeed)
    (else
      ;[1 1 1] If not char, check if we hit respawn trigger
      (bind _hitresult_2 (CallFunction|CheckRespawnHit _returnvalue))
      (if _hitresult_2
        (goto _label)))))

(event EventTick
  (params (DeltaSeconds :type Float%20%28single-precision%29))
  (|CallParentFunction 0.0))

(event EventBeginPlay
  ;[1 1 1] Liikkuuko vertikaalisesti
  (Variables|Default|SetDropsVertically false)
  ;[1 1 1] Määrittelee skaalauksen ja nopeuden vaihteluvälin ja liikkeen suunnan
  (Variables|Default|SetDefaultScale 0.2)
  (Variables|Default|SetMinScale 1.0)
  (Variables|Default|SetMaxScale 2.0)
  (Variables|Default|SetDefaultSpeed "-5.000000, 0,0.000000")
  (Variables|Default|SetSpeedVariance 1.5))

(fn ConstructionScript
  ;[1 1 1] Initial position ja speed
  (Variables|Default|SetSpeed "-5.000000, 0,0.000000")
  (Variables|Default|SetInitialPosition "1300.000000,0.000000,500.000000"))